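; Gameplay ability that casts a fireball from the character, committing the ability and starting its UI cooldown on activation.
; It plays the fireball montage, then waits for the Skill.fireball.spawn gameplay event to spawn BP_Fireball at the mesh's FireballSocket.
; The projectile receives the caster as instigator and an outgoing GE_DashDamage effect spec.
; The ability ends after spawning or when the montage is interrupted or cancelled.
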(event `self.K2_ActivateAbility`
  (`self.K2_CommitAbility`)
  (`self.DoUICooldown`)
  (`AbilityTask_PlayMontageAndWait.CreatePlayMontageAndWaitProxy` "None" "/Game/Blueprints/Characters/Animation/AM_Fireball.AM_Fireball"
    (:`then`
      (`AbilityTask_WaitGameplayEvent.WaitGameplayEvent` (struct :`TagName` "skill.fireball.spawn") null
        (:`EventReceived`
          (bind _characterbase (`self.GetPlayerCharacteristics`))
          (`|SpawnActorFromClass` "/Game/Blueprints/Characters/GameplayAbilities/Fireball/BP_Fireball.BP_Fireball_C" (`SceneComponent.GetSocketTransform` (`Character.Mesh` _characterbase) "FireballSocket" "RTS_World") "AlwaysSpawn" "OverrideRootScale" null (`self.MakeOutgoingGameplayEffectSpec` "/Game/Blueprints/Characters/GameplayAbilities/Dash/GE_DashDamage.GE_DashDamage_C") _characterbase)
          (`self.K2_EndAbility`))))
    (:`OnInterrupted`
      (`self.K2_EndAbility` :!label _label))
    (:`OnCancelled`
      (goto _label))))