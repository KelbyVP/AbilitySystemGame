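; Base gameplay ability Blueprint that links abilities to the player's cooldown UI; its activate and end events are unimplemented.
; GetPlayerCharacteristics resolves the owning BP_CharacterBase and its BP_PlayerController, if any.
; DoUICooldown uses that controller to walk the primary UI's slots and start the cooldown on those whose ability class matches this ability's info.
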(fn `DoUICooldown`
  (bind (_characterbase _controllerbase) (`self.GetPlayerCharacteristics`))
  (`/Engine/EditorBlueprintResources/StandardMacros.IsValid` _controllerbase
    (:`Is Valid`
      (for _array_element (`/Game/UI/WBP_PrimaryUI.Slots` (`/Game/Blueprints/BP_PlayerController.PrimaryUI` _controllerbase))
        (bind _returnvalue (`self.GetAbilityInfo`))
        (bind (_abilityinfo_cooldownduration _abilityinfo_cost _abilityinfo_costtype _abilityinfo_uimat _abilityinfo_abilityclass) (break `GameplayAbilityInfo` (`/Game/UI/WBP_AbilitySlot.AbilityInfo` _array_element)))
        (if (== (`.AbilityClass` (break `GameplayAbilityInfo` _returnvalue)) _abilityinfo_abilityclass)
          (`/Game/UI/WBP_AbilitySlot.StartCooldown` _array_element))))))

(fn `GetPlayerCharacteristics`
  (returns (CharacterBase :type "/Game/Blueprints/Characters/BP_CharacterBase Object Reference") (ControllerBase :type "/Game/Blueprints/BP_PlayerController Object Reference"))
  (bind _asbp_character_base (cast `/Game/Blueprints/Characters/BP_CharacterBase` (`self.GetOwningActorFromActorInfo`)))
  (bind _asbp_player_controller (cast `/Game/Blueprints/BP_PlayerController` (`Pawn.GetController` _asbp_character_base))
    (:`then`
      _)
    (:`CastFailed`
      _))
  (return _asbp_character_base _asbp_player_controller))