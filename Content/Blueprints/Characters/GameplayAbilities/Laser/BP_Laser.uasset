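; BP_Laser is a laser beam actor for a character gameplay ability, with a skeletal mesh that stretches to a variable length.
; BeginPlay records the original beam length from the actor to the mesh's "end" socket.
; Each Tick measures the distance from the actor to LaserEndDetector and passes the difference from the original length to AnimBP_LaserSkeleton as an X-axis EndBoneOffset, so bone displacement sets the beam's length.
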(event `self.ReceiveTick`
  (params (DeltaSeconds :type "Float (single-precision)"))
  (bind _asanim_bp_laser_skeleton (cast `/Game/Blueprints/Characters/GameplayAbilities/Laser/LaserAssets/AnimBP_LaserSkeleton` (`SkeletalMeshComponent.GetAnimInstance` (`self.LaserMesh`))))
  (set `/Game/Blueprints/Characters/GameplayAbilities/Laser/LaserAssets/AnimBP_LaserSkeleton.EndBoneOffset` (`KismetMathLibrary.MakeVector` (- (`KismetMathLibrary.VSize` (- (`SceneComponent.K2_GetComponentLocation` (`self.LaserEndDetector`)) (`self.K2_GetActorLocation`))) (`self.BeamOriginalLength`))) _asanim_bp_laser_skeleton))

(event `self.ReceiveBeginPlay`
  (set `self.BeamOriginalLength` (`KismetMathLibrary.VSize` (- (`SceneComponent.GetSocketLocation` (`self.LaserMesh`) "end") (`self.K2_GetActorLocation`)))))

(fn `UserConstructionScript`)