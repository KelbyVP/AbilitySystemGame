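; GA_Laser is a channeled laser ability that damages and pushes back the characters it hits.
; It plays a casting montage, spawns BP_Laser on the mesh's LaserSocket after a short delay, and enables camera control rotation.
; Each deal-damage gameplay event applies GE_LaserDamage and a stunning push away from the beam end, or ends the ability if cost runs out.
; Ending removes the draining cost effect, destroys the laser and restores rotation.
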(event `self.K2_ActivateAbility`
  (`self.K2_CommitAbility`)
  (`self.DoUICooldown`)
  (`AbilityTask_PlayMontageAndWait.CreatePlayMontageAndWaitProxy` "None" "/Game/Blueprints/Characters/Animation/AM_LaserCasting.AM_LaserCasting" 1.0 "Start"
    (:`then`
      (`KismetSystemLibrary.Delay` 0.2)
      (bind _characterbase (`self.GetPlayerCharacteristics`))
      (bind (_asynctaskproxy _spawnedactor) (`AbilityTask_SpawnActor.SpawnActor` (struct) "/Game/Blueprints/Characters/GameplayAbilities/Laser/BP_Laser.BP_Laser_C" _characterbase)
        (:`then`
          (bind _output_get (set `self.LaserActor` _spawnedactor))
          (`Actor.K2_AttachToComponent` _output_get (`Character.Mesh` _characterbase) "LaserSocket" "SnapToTarget" "SnapToTarget" "KeepRelative" true)
          (`/Game/Blueprints/Characters/BP_CharacterBase.MakeCameraControlRotation` _characterbase true)
          (bind (_asynctaskproxy_2 _payload) (`AbilityTask_WaitGameplayEvent.WaitGameplayEvent` (struct :`TagName` "skill.laser.dealDamage") null)
            (:`EventReceived`
              (bind _bcoststillavailable (`self.IsCostStillAvailable`))
              (if _bcoststillavailable
                (bind (_eventtag _instigator _target _optionalobject _optionalobject2 _contexthandle _instigatortags _targettags _eventmagnitude _targetdata) (break `GameplayEventData` _payload))
                (`self.BP_ApplyGameplayEffectToTarget` _targetdata "/Game/Blueprints/Characters/GameplayAbilities/Laser/GE_LaserDamage.GE_LaserDamage_C")
                (for _array_element (`AbilitySystemBlueprintLibrary.GetActorsFromTargetData` _targetdata)
                  (bind _asbp_character_base (cast `/Game/Blueprints/Characters/BP_CharacterBase` _array_element))
                  (`/Game/Blueprints/Characters/BP_CharacterBase.PushCharacter` _asbp_character_base (`KismetMathLibrary.Normal` (- (`Actor.K2_GetActorLocation` _asbp_character_base) (`SceneComponent.K2_GetComponentLocation` (`/Game/Blueprints/Characters/GameplayAbilities/Laser/BP_Laser.LaserEndDetector` (cast `/Game/Blueprints/Characters/GameplayAbilities/Laser/BP_Laser` (`self.LaserActor`) :!pure true))))) 500.0 0.3))
                (else
                  (`self.K2_EndAbility`))))))))
    (:`OnCompleted`
      (`self.K2_EndAbility` :!label _label))
    (:`OnBlendOut`
      (goto _label))
    (:`OnInterrupted`
      (goto _label))
    (:`OnCancelled`
      (goto _label))))

(event `self.K2_OnEndAbility`
  (params (bWasCancelled :type Boolean))
  (`self.BP_RemoveGameplayEffectFromOwnerWithAssetTags` (struct :`GameplayTags` (struct :`(TagName` "skill.laser.drainingCost"))))
  (`Actor.K2_DestroyActor` (`self.LaserActor`))
  (bind _characterbase (`self.GetPlayerCharacteristics`))
  (`/Game/Blueprints/Characters/BP_CharacterBase.MakeCameraControlRotation` _characterbase false))